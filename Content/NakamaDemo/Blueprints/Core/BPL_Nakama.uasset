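; Blueprint function library of shared helpers for the Nakama demo.
; Getters fetch the user session, Nakama client and realtime client by casting player controller 0 to NakamaDemoController.
; Error helpers print Nakama and realtime error messages with their codes in red on screen.
; Formatting helpers map message severity to a color and turn a DateTime into a readable date and time string.
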(fn `Clean Date Time to String`
  (params (InDateTime :type "DateTime Structure"))
  (returns (NewParam :type String))
  (bind (_year _month _day _hour _minute _second) (`KismetMathLibrary.BreakDateTime` InDateTime))
  (return (`KismetTextLibrary.Conv_TextToString` (`|FormatText` "{year}.{month}.{day} - {hour}:{minute}:{second} " (`KismetTextLibrary.Conv_IntToText` _year false false 2) (`KismetTextLibrary.Conv_IntToText` _month false true 2) (`KismetTextLibrary.Conv_IntToText` _day false true 2) (`KismetTextLibrary.Conv_IntToText` _hour false true 2) (`KismetTextLibrary.Conv_IntToText` _minute false true 2) (`KismetTextLibrary.Conv_IntToText` _second false true 2)))))

(fn `GetCurrentSession`
  (returns (Session :type "NakamaSession Object Reference"))
  (bind _asnakama_demo_controller (cast `/Game/NakamaDemo/Blueprints/Core/NakamaDemoController` (`GameplayStatics.GetPlayerController` null)))
  (return (`/Game/NakamaDemo/Blueprints/Core/NakamaDemoController.UserSession` _asnakama_demo_controller)))

(fn `GetNakamaClient`
  (returns (NakamaClient :type "NakamaClient Object Reference"))
  (bind _asnakama_demo_controller (cast `/Game/NakamaDemo/Blueprints/Core/NakamaDemoController` (`GameplayStatics.GetPlayerController` null)))
  (return (`/Game/NakamaDemo/Blueprints/Core/NakamaDemoController.NakamaClient` _asnakama_demo_controller)))

(fn `GetNakamaRealtimeClient`
  (returns (NakamaRealtimeClient :type "NakamaRealtimeClient Object Reference"))
  (bind _asnakama_demo_controller (cast `/Game/NakamaDemo/Blueprints/Core/NakamaDemoController` (`GameplayStatics.GetPlayerController` null)))
  (return (`/Game/NakamaDemo/Blueprints/Core/NakamaDemoController.NakamaRealtimeClient` _asnakama_demo_controller)))

(fn `PrintNakamaError`
  (params (Error :type "NakamaError Structure"))
  (bind (_message _code) (break `NakamaError` Error))
  (`KismetSystemLibrary.PrintString` null (`KismetStringLibrary.Concat_StrStr` "Nakama Error: " _message " Code: " (`|GetEnumeratorNameAsString` _code)) true true (struct :`R` 1.0 :`A` 1.0)))

(fn `PrintNakamaRealtimeError`
  (params (RealtimeError :type "NakamaRtError Structure"))
  (bind (_message _code) (break `NakamaRtError` RealtimeError))
  (`KismetSystemLibrary.PrintString` null (`KismetStringLibrary.Concat_StrStr` "Nakama Error: " _message " Code: " (`|GetEnumeratorNameAsString` _code)) true true (struct :`R` 1.0 :`A` 1.0)))

(fn `SeverityToColor`
  (params (Severity :type "/Game/NakamaDemo/Blueprints/Enums/ENotificationSeverity Enum" :default "NewEnumerator0"))
  (returns (NewParam :type "LinearColor Structure"))
  (switch `/Game/NakamaDemo/Blueprints/Enums/ENotificationSeverity` Severity
    (:`NewEnumerator0`
      (return (struct :`R` 0.015209 :`G` 0.0185 :`B` 0.022174 :`A` 1.0)))
    (:`NewEnumerator1`
      (return (struct :`R` 1.0 :`G` 0.027806 :`A` 1.0)))
    (:`NewEnumerator2`
      (return (struct :`G` 0.775369 :`B` 1.0 :`A` 1.0)))
    (:`NewEnumerator3`
      (return (struct :`R` 1.0 :`G` 0.820607 :`A` 1.0)))
    (:`NewEnumerator4`
      (return (struct :`G` 1.0 :`B` 0.280401 :`A` 1.0)))))